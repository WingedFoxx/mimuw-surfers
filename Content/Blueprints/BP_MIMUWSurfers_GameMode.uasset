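; MIMUW Surfers game mode that runs the main HUD, distance score and game-over screen.
; BeginPlay builds the HUD and distance timer, retries the surfer character cast until it succeeds, then runs that HUD and timer setup again.
; The looping timer turns the character's X position into Distance and updates the HUD.
; GameOver shows that score in a widget created only if none exists; AddCoins is an empty stub.
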(event Custom|UpdateDistance
  (bind _returnvalue (Utilities|Time|SetTimerbyEvent (delegate Custom|Add%20Score) 0.1 true))
  (Variables|Default|SetDistanceTimer _returnvalue))

(event Custom|Add%20Score
  (Variables|Default|SetDistance (/ (Math|Float|Round (.x (Transformation|GetActorLocation (Variables|Default|GetAs%20BP%20Surfer%20Character)))) 10))
  (Rendering|Components|TextRender|SetText (Variables|/Game/UserWidget/MainHUD_UI.MainHUD_UI_C|GetDistanceValueTxt (Variables|Default|GetMain%20Hud%20UI)) (Utilities|Text|ToText(Integer) (Variables|Default|GetDistance))))

(event EventBeginPlay
  (Utilities|FlowControl|Sequence
    (:then_0
      _)
    (:then_1
      (bind _asbp_surfer_character (Utilities|Casting|CastToBP_SurferCharacter (Game|GetPlayerCharacter 0) :!label _label)
        (:then
          (Variables|Default|SetAs%20BP%20Surfer%20Character _asbp_surfer_character))
        (:CastFailed
          (Utilities|FlowControl|Delay 0.01)
          (goto _label)))))
  (bind _returnvalue (UserInterface|CreateWidget "/Game/UserWidget/MainHUD_UI.MainHUD_UI_C"))
  (bind _output_get (Variables|Default|SetMain%20Hud%20UI _returnvalue))
  (UserInterface|Viewport|AddtoViewport _output_get 0)
  (CallFunction|UpdateDistance))

(event EventTick
  (params (DeltaSeconds :type Float%20%28single-precision%29)))

(event EventGameOver
  (Variables|Default|GetGameOver%20UI
    (:then)
    (:else
      (bind _returnvalue (UserInterface|CreateWidget "/Game/UserWidget/GameOver_UI.GameOver_UI_C"))
      (bind _output_get (Variables|Default|SetGameOver%20UI _returnvalue))
      (UserInterface|Viewport|AddtoViewport _output_get 0)
      (Default|SetScoresTxt (Variables|Default|GetGameOver%20UI) 0 (Variables|Default|GetDistance)))))

(fn ConstructionScript)

(fn AddCoins
  (params (Value :type Integer))
  (return))